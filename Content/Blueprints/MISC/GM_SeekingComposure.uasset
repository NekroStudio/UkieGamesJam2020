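; GM_SeekingComposure, which appears to be a game mode by its prefix, tracks elapsed gameplay time and holds a reference to the player character.
; On BeginPlay it starts a looping one-second timer that increments GameplayTimer, keeps the timer handle, and caches player 0's character cast to BP_PlayerCharacter.
; EndLevel only prints a level-complete message and leaves the timer running.
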(event Custom|StartGameplayTimer
  (bind _returnvalue (Utilities|Time|SetTimerbyEvent (delegate Custom|IncreaseTimer) 1.0 true))
  (Variables|Default|SetGameplayTimerHandle _returnvalue))

(event Custom|IncreaseTimer
  (Math|Integer|IncrementInt (Variables|Default|GetGameplayTimer)))

(event Custom|EndLevel
  (Development|PrintString "LevelComplete"))

(event EventBeginPlay
  (CallFunction|StartGameplayTimer)
  (CallFunction|FStoreCharacterRef))

(fn ConstructionScript)

(fn FStoreCharacterRef
  (Variables|Default|SetCharacter (.AsBP%20Player%20Character (Utilities|Casting|CastToBP_PlayerCharacter (Game|GetPlayerCharacter 0)))))