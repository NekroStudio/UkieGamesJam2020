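; Player character for Seeking Composure, handling movement, inventory, points, hold-to-zoom inspection and an anxiety mechanic.
; A looping timer raises anxiety; holding listen-to-music roots the player and lowers it, with a re-use delay after release.
; High anxiety triggers camera shakes, slower movement and a timed random roll for panic attacks that freeze movement.
; Event dispatchers broadcast input and state changes, and the HUD widget is initialized with this character.
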(event Custom|ItemType
  (params (Item :type BP%20Pickup%20Interactable%20Object%20Reference))
  (Variables|Default|SetCurrentItemType Item))

(event Custom|AddToInventory
  (params (ItemToAdd :type BP%20Base%20Interactables%20Class%20Reference))
  ;[1 1 1] Inventory
  (Utilities|Array|Add (Variables|Default|GetInventory) ItemToAdd)
  (Development|PrintString (Utilities|String|Append "Added Item: " (Utilities|GetClassDisplayName ItemToAdd))))

(event Custom|ZoomOut
  (bind _springarm (Variables|Default|GetSpringArm))
  ;[1 1 1] Zoom/Inspect Mechanic
  (Variables|/Script/Engine.SpringArmComponent|SetTargetArmLength _springarm (Math|Float|Clamp(Float) (+ (Variables|/Script/Engine.SpringArmComponent|GetTargetArmLength _springarm) 2.5) -5e+01 5e+01))
  (if (== (Math|Float|Clamp(Float) (+ (Variables|/Script/Engine.SpringArmComponent|GetTargetArmLength _springarm) 2.5) -5e+01 5e+01) 0.0)
    (Utilities|Time|ClearandInvalidateTimerbyHandle (Variables|Zoom|GetZoomOutTimerHandle))
    (Variables|/Script/Engine.CharacterMovementComponent|SetMaxWalkSpeed (Variables|Character|GetCharacterMovement) (Variables|Default|GetBaseMaxMoveSpeed))))

(event Custom|ZoomIn
  (bind _springarm (Variables|Default|GetSpringArm))
  ;[1 1 1] Zoom/Inspect Mechanic
  (Variables|/Script/Engine.SpringArmComponent|SetTargetArmLength _springarm (Math|Float|Clamp(Float) (- (Variables|/Script/Engine.SpringArmComponent|GetTargetArmLength _springarm) 2.5) -5e+01 5e+01))
  (CallFunction|FPlayerSpeedwhenZoomed))

(event Custom|TriggerAnxietyBar
  ;[1 1 1] AnxietyBar/Panic Attack
  (bind _returnvalue (Utilities|Time|SetTimerbyEvent (delegate Custom|IncreaseAnxiety) (Variables|AnxietyVars|GetAnxietyIncreaseLoopTime) true))
  (Variables|AnxietyVars|SetAnxietyBarTimerHandle _returnvalue))

(event Custom|CheckPanicAttack
  (bind _panicattacktimerhandle (Variables|AnxietyVars|GetPanicAttackTimerHandle))
  ;[1 1 1] AnxietyBar/Panic Attack
  ;;[1 1 1] Trigger Potential Panic Attack
  (if (== (Math|Random|RandomIntegerinRange 0 20) (Variables|AnxietyVars|GetPanicAttackNumber))
    (Variables|AnxietyVars|SetHavingPanicAttack true)
    (Default|CallEDHavingPanicAttack)
    (Variables|/Script/Engine.CharacterMovementComponent|SetMaxWalkSpeed (Variables|Character|GetCharacterMovement) 0.0)
    (CallFunction|FPanicCamShake)
    (else
      (if (Variables|AnxietyVars|GetHavingPanicAttack)
        (Utilities|Time|PauseTimerbyHandle _panicattacktimerhandle)
        (Utilities|FlowControl|Delay 5.0)
        (Utilities|Time|UnpauseTimerbyHandle _panicattacktimerhandle))
      (Default|CallEDPotentialPanicAttack)
      (CallFunction|F70%CamShake)
      (Variables|AnxietyVars|SetHavingPanicAttack false)
      (Variables|/Script/Engine.CharacterMovementComponent|SetMaxWalkSpeed (Variables|Character|GetCharacterMovement) 4.5e+02))))

(event Custom|TriggerPotentialPanicAttack
  ;[1 1 1] AnxietyBar/Panic Attack
  ;;[1 1 1] Trigger Potential Panic Attack
  (bind _returnvalue (Utilities|Time|SetTimerbyEvent (delegate Custom|CheckPanicAttack) 1.0 true))
  (Variables|AnxietyVars|SetPanicAttackTimerHandle _returnvalue)
  (Variables|/Script/Engine.CharacterMovementComponent|SetMaxWalkSpeed (Variables|Character|GetCharacterMovement) 4.5e+02))

(event Custom|IncreaseAnxiety
  ;[1 1 1] AnxietyBar/Panic Attack
  (bind _output_get (Variables|AnxietyVars|SetAnxietyBar (Math|Float|Clamp(Float) (+ (Variables|AnxietyVars|GetAnxietyBar) (Variables|AnxietyVars|GetIncreaseAmount)) 0.0 1e+02)))
  (Default|CallEDUpdateAnxiety (/ _output_get (Variables|AnxietyVars|GetMaxAnxiety)))
  (if (>= _output_get 7e+01)
    (if (Variables|AnxietyVars|GetHavingPanicAttack)
      (CallFunction|FPanicCamShake)
      (else
        (CallFunction|F70%CamShake)
        (Utilities|FlowControl|Sequence
          (:then_0
            (Utilities|FlowControl|DoOnce false :!label _label
              (:Completed
                (CallFunction|TriggerPotentialPanicAttack)
                (Default|CallEDPotentialPanicAttack))))
          (:then_1
            (Default|CallEDPotentialPanicAttack)
            (if (>= _output_get 1e+02)
              (Variables|/Script/Engine.CharacterMovementComponent|SetMaxWalkSpeed (Variables|Character|GetCharacterMovement) 2.5e+02))))))
    (else
      (Utilities|Time|ClearandInvalidateTimerbyHandle (Variables|AnxietyVars|GetPanicAttackTimerHandle))
      (Variables|/Script/Engine.CharacterMovementComponent|SetMaxWalkSpeed (Variables|Character|GetCharacterMovement) (Variables|Default|GetBaseMaxMoveSpeed))
      (Default|CallEDNoPotentialPanicAttack)
      (goto _label Reset))))

(event Custom|DecreaseAnxiety
  ;[1 1 1] Listening to music to decrease anxiety
  (bind _output_get (Variables|AnxietyVars|SetAnxietyBar (Math|Float|Clamp(Float) (- (Variables|AnxietyVars|GetAnxietyBar) (Variables|AnxietyVars|GetDecreaseAmount)) 0.0 1e+02)))
  (Default|CallEDUpdateAnxiety (/ _output_get (Variables|AnxietyVars|GetMaxAnxiety)))
  (Variables|/Script/Engine.CharacterMovementComponent|SetMaxWalkSpeed (Variables|Character|GetCharacterMovement) 0.0))

(event EventBeginPlay
  ;[1 1 1] Begin play
  (Variables|Default|SetBaseMaxMoveSpeed (Variables|/Script/Engine.CharacterMovementComponent|GetMaxWalkSpeed (Variables|Character|GetCharacterMovement)))
  (CallFunction|TriggerAnxietyBar)
  (CallFunction|FCreateWidget)
  (bind _outactors (Actor|GetAllActorsOfClass "/Game/Blueprints/Interactables/BP_PickupInteractable.BP_PickupInteractable_C"))
  (for _array_element _outactors
    (EventDispatchers|BindEventtoEDItemType _array_element (delegate Custom|ItemType))))

(event EventIPointsIncrease
  (params (IncreasePoints :type Integer))
  (bind _output_get (Variables|Default|SetPoints (+ (Variables|Default|GetPoints) IncreasePoints)))
  (Development|PrintString (Utilities|String|Append "CurrentPoints: " (Utilities|String|ToString(Integer) _output_get) " Timer: " (Utilities|String|ToString(Integer) (Variables|/Game/Blueprints/MISC/GM_SeekingComposure.GM_SeekingComposure_C|GetGameplayTimer (.AsGM%20Seeking%20Composure (Utilities|Casting|CastToGM_SeekingComposure (Game|GetGameMode)))))) true true "(R=1.000000,G=0.013544,B=0.000000,A=1.000000)"))

(event Input|ActionEvents|InputActionInteract
  (params (Key :type Key%20Structure :default "None"))
  ;[1 1 1] Interact
  (:Pressed
    (Default|CallEDInteractPressed)))

(event Input|ActionEvents|InputActionZoomInspect
  (params (Key :type Key%20Structure :default "None"))
  ;[1 1 1] Zoom/Inspect Mechanic
  (:Pressed
    (Variables|Zoom|SetZoomHeld true)
    (bind _returnvalue (Utilities|Time|SetTimerbyEvent (delegate Custom|ZoomIn) (Utilities|Time|GetWorldDeltaSeconds) true))
    (Variables|Zoom|SetZoomInTimerHandle _returnvalue)
    (Default|CallEDZoomDown (Variables|Zoom|GetZoomHeld)))
  (:Released
    (Variables|Zoom|SetZoomHeld false)
    (Utilities|Time|ClearandInvalidateTimerbyHandle (Variables|Zoom|GetZoomInTimerHandle))
    (bind _returnvalue_2 (Utilities|Time|SetTimerbyEvent (delegate Custom|ZoomOut) (Utilities|Time|GetWorldDeltaSeconds) true))
    (Variables|Zoom|SetZoomOutTimerHandle _returnvalue_2)
    (Default|CallEDZoomDown (Variables|Zoom|GetZoomHeld))))

(event Input|ActionEvents|InputActionPause
  (params (Key :type Key%20Structure :default "None"))
  ;[1 1 1] Controls
  (:Pressed
    (Default|CallEDPaused))
  (:Released
    (Default|CallEDUnpaused)))

(event Input|ActionEvents|InputActionListentoMusic
  (params (Key :type Key%20Structure :default "None"))
  ;[1 1 1] Listening to music to decrease anxiety
  (:Pressed
    (if (Variables|AnxietyVars|GetCanListenToMusic)
      (bind _returnvalue (Utilities|Time|SetTimerbyEvent (delegate Custom|DecreaseAnxiety) (Variables|AnxietyVars|GetAnxietyIncreaseLoopTime) true))
      (Variables|AnxietyVars|SetDecreaseAnxietyTimerHandle _returnvalue)
      (Default|CallEDListeningtoMusic)
      (Utilities|Time|ClearandInvalidateTimerbyHandle (Variables|AnxietyVars|GetAnxietyBarTimerHandle))
      (Variables|AnxietyVars|SetCanListenToMusic false)))
  (:Released
    (Utilities|Time|ClearandInvalidateTimerbyHandle (Variables|AnxietyVars|GetDecreaseAnxietyTimerHandle))
    (Variables|/Script/Engine.CharacterMovementComponent|SetMaxWalkSpeed (Variables|Character|GetCharacterMovement) (Variables|Default|GetBaseMaxMoveSpeed))
    (Default|CallEDStoppedListeningtoMusic)
    (CallFunction|TriggerAnxietyBar)
    (Utilities|FlowControl|Delay 5.0)
    (Variables|AnxietyVars|SetCanListenToMusic true)))

(event Input|ActionEvents|InputActionLMBDown
  (params (Key :type Key%20Structure :default "None"))
  ;[1 1 1] LMB
  (:Pressed
    (Default|CallEDLMBDown)))

(event Input|AxisEvents|InputAxisForwards/Backwards
  (params (AxisValue :type Float%20%28single-precision%29))
  ;[1 1 1] Controls
  (Pawn|Input|AddMovementInput (Math|Vector|GetForwardVector (Variables|Character|GetMesh)) AxisValue false))

(event Input|AxisEvents|InputAxisLeft/Right
  (params (AxisValue :type Float%20%28single-precision%29))
  ;[1 1 1] Controls
  (Pawn|Input|AddMovementInput (Math|Vector|GetRightVector (Variables|Character|GetMesh)) AxisValue false))

(event Input|AxisEvents|InputAxisMouse/GamepadLookUp
  (params (AxisValue :type Float%20%28single-precision%29))
  ;[1 1 1] Controls
  (Pawn|Input|AddControllerPitchInput AxisValue)
  (Default|CallEDLookUp AxisValue))

(event Input|AxisEvents|InputAxisMouse/GamepadTurn
  (params (AxisValue :type Float%20%28single-precision%29))
  ;[1 1 1] Controls
  (Pawn|Input|AddControllerYawInput AxisValue)
  (Default|CallEDTurn AxisValue))

(fn ConstructionScript)

(fn FPlayerSpeedwhenZoomed
  (bind _charactermovement (Variables|Character|GetCharacterMovement))
  (if (Variables|Zoom|GetZoomHeld)
    (Variables|/Script/Engine.CharacterMovementComponent|SetMaxWalkSpeed _charactermovement 0.0)
    (else
      (Variables|/Script/Engine.CharacterMovementComponent|SetMaxWalkSpeed _charactermovement (Variables|Default|GetBaseMaxMoveSpeed)))))

(fn FCreateWidget
  (bind _returnvalue (UserInterface|CreateWidget "/Game/Alex/W_HUDManager.W_HUDManager_C"))
  (Variables|Default|SetHUDRef _returnvalue)
  (UserInterface|Viewport|AddtoViewport _returnvalue 0)
  (Default|Init _returnvalue self))

(fn F70%CamShake
  (Camera|PlayWorldCameraShake "/Game/Blueprints/BP_AnxietyCamShake.BP_AnxietyCamShake_C" (Transformation|GetActorLocation) 0.0 5e+02))

(fn FPanicCamShake
  (Camera|PlayWorldCameraShake "/Game/Blueprints/BP_PanicAttackCamShake.BP_PanicAttackCamShake_C" (Transformation|GetActorLocation) 0.0 5e+02))