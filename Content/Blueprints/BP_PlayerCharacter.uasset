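; BP_PlayerCharacter is the player character, handling basic movement and look input.
; Forward/backward and left/right axes add movement along the Camera's forward and right vectors, so movement follows the view direction.
; Mouse/gamepad look axes feed controller pitch and yaw directly, with no scaling in the graph.
; The construction script is empty.
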(event Input|AxisEvents|InputAxisForwards/Backwards
  (params (AxisValue :type Float%20%28single-precision%29))
  (Pawn|Input|AddMovementInput (Math|Vector|GetForwardVector (Variables|Default|GetCamera)) AxisValue false))

(event Input|AxisEvents|InputAxisLeft/Right
  (params (AxisValue :type Float%20%28single-precision%29))
  (Pawn|Input|AddMovementInput (Math|Vector|GetRightVector (Variables|Default|GetCamera)) AxisValue false))

(event Input|AxisEvents|InputAxisMouse/GamepadLookUp
  (params (AxisValue :type Float%20%28single-precision%29))
  (Pawn|Input|AddControllerPitchInput AxisValue))

(event Input|AxisEvents|InputAxisMouse/GamepadTurn
  (params (AxisValue :type Float%20%28single-precision%29))
  (Pawn|Input|AddControllerYawInput AxisValue))

(fn ConstructionScript)