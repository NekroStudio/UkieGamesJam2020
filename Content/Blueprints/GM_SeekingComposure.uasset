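; Game mode Blueprint for SeekingComposure that tracks elapsed gameplay time.
; On BeginPlay it caches the player character as BP_PlayerCharacter and starts a looping one-second timer, keeping its handle.
; Each tick of that timer increments a gameplay counter and prints it on screen as debug text.
; The cached character reference is not used elsewhere in the graph.
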(event Custom|GametimeCounter
  (bind _result (Math|Float|IncrementFloat (Variables|Default|GetGameplayTimer))
    (:%20%20
      (Development|PrintString (Utilities|String|ToString(Float) _result) true true "(R=1.000000,G=0.000000,B=0.853594,A=1.000000)"))))

(event Custom|StartGameplaytimer
  (bind _returnvalue (Utilities|Time|SetTimerbyEvent (delegate Custom|GametimeCounter) 1.0 true))
  (Variables|Default|SetGameplayTimerHandle _returnvalue))

(event EventBeginPlay
  (Variables|Default|SetCharacter (.AsBP%20Player%20Character (Utilities|Casting|CastToBP_PlayerCharacter (Game|GetPlayerCharacter 0))))
  (CallFunction|StartGameplaytimer))

(fn ConstructionScript)