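; Base interactable pickup that the player collects into their inventory by zooming inside its collision volume and pressing interact.
; Overlap starts a per-frame looping timer that checks the zoom state bound from the character, then after a delay enables interaction, lights a point light and fires dispatchers.
; Interacting maps the item name to an item class, adds it to the inventory, broadcasts the collection and destroys the actor.
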(event OnComponentBeginOverlap(Collision)
  (params (OverlappedComponent :type Primitive%20Component%20Object%20Reference) (OtherActor :type Actor%20Object%20Reference) (OtherComp :type Primitive%20Component%20Object%20Reference) (OtherBodyIndex :type Integer) (bFromSweep :type Boolean) (SweepResult :type Hit%20Result%20Structure%20%28by%20ref%29))
  ;[1 1 1] Begin and end overlap
  (Utilities|IsPlayerCharacter OtherActor
    (:IsPlayer
      (Variables|BaseVariables|SetInVolume true)
      (Input|EnableInput (Game|GetPlayerController 0))
      (bind _returnvalue (Utilities|Time|SetTimerbyEvent (delegate Custom|CheckZoom) (Utilities|Time|GetWorldDeltaSeconds) true))
      (Variables|BaseVariables|SetZoomTimerHandle _returnvalue))))

(event OnComponentEndOverlap(Collision)
  (params (OverlappedComponent :type Primitive%20Component%20Object%20Reference) (OtherActor :type Actor%20Object%20Reference) (OtherComp :type Primitive%20Component%20Object%20Reference) (OtherBodyIndex :type Integer))
  ;[1 1 1] Begin and end overlap
  (Utilities|IsPlayerCharacter OtherActor
    (:IsPlayer
      (Variables|BaseVariables|SetInVolume false)
      (Variables|BaseVariables|SetAbleToInteract false)
      (CallFunction|ToggleLightOff)
      (Default|CallEDCannotInteract))))

(event Custom|CanInteract
  ;[1 1 1] Interact with object if in volume and interact is pressed
  (if (Variables|BaseVariables|GetInVolume)
    (if (Variables|BaseVariables|GetAbleToInteract)
      (CallFunction|FPassItemtoCharacter)
      (Utilities|FlowControl|Delay 0.01)
      (Actor|DestroyActor))))

(event Custom|ZoomDown?
  (params (IsHeld :type Boolean))
  ;[1 1 1] ZoomBindEvent
  (Variables|BaseVariables|SetCharacterZoomed IsHeld))

(event Custom|ToggleLightOn
  ;[1 1 1] Change Light Intensity
  (Rendering|Components|Light|SetIntensity (Variables|Default|GetPointLight) 5e+03))

(event Custom|ToggleLightOff
  ;[1 1 1] Change Light Intensity
  (Rendering|Components|Light|SetIntensity (Variables|Default|GetPointLight) 0.0))

(event Custom|CheckZoom
  ;[1 1 1] Begin and end overlap
  (if (Variables|BaseVariables|GetCharacterZoomed)
    (Utilities|FlowControl|Delay (Variables|Default|GetCanInteractDelay))
    (Variables|BaseVariables|SetAbleToInteract true)
    (CallFunction|ToggleLighton)
    (Default|CallEDCanInteract)
    (Default|CallEDItemType self)
    (elif (not (Variables|BaseVariables|GetInVolume))
      (Utilities|Time|ClearandInvalidateTimerbyHandle (Variables|BaseVariables|GetZoomTimerHandle))
      (CallFunction|ToggleLightOff)
      (Default|CallEDCannotInteract))))

(event EventBeginPlay
  ;[1 1 1] Begin play, get refs and bind interact
  (CallFunction|FGetRefs)
  (CallFunction|FBindings))

(fn ConstructionScript)

(fn FGetRefs
  (Variables|Default|SetCharacter (.AsBP%20Player%20Character (Utilities|Casting|CastToBP_PlayerCharacter (Game|GetPlayerCharacter 0))))
  (return))

(fn FBindings
  (bind _character (Variables|Default|GetCharacter))
  (EventDispatchers|BindEventtoEDInteractPressed _character (EventDispatchers|CreateEvent :!event Custom|CanInteract))
  (EventDispatchers|BindEventtoEDZoomDown _character (EventDispatchers|CreateEvent :!event Custom|ZoomDown?)))

(fn FPassItemtoCharacter
  (switch Utilities|FlowControl|Switch|SwitchonE_ItemName (Variables|Default|GetItemName)
    (:NewEnumerator0
      (Default|AddtoInventory (Variables|Default|GetCharacter) "/Game/Blueprints/Interactables/1LivingRoomItems/BP_Notebook.BP_Notebook_C")
      (Default|CallEDItemCollected "/Game/Blueprints/Interactables/1LivingRoomItems/BP_Notebook.BP_Notebook_C" (Variables|Default|GetItemNameString)))
    (:NewEnumerator3
      (Default|AddtoInventory (Variables|Default|GetCharacter) "/Game/Blueprints/Interactables/1LivingRoomItems/BP_Backpack.BP_Backpack_C")
      (Default|CallEDItemCollected "/Game/Blueprints/Interactables/1LivingRoomItems/BP_Backpack.BP_Backpack_C" (Variables|Default|GetItemNameString)))
    (:NewEnumerator1
      (Default|AddtoInventory (Variables|Default|GetCharacter) "/Game/Blueprints/Interactables/1LivingRoomItems/BP_Keys.BP_Keys_C")
      (Default|CallEDItemCollected "/Game/Blueprints/Interactables/1LivingRoomItems/BP_Keys.BP_Keys_C" (Variables|Default|GetItemNameString)))
    (:NewEnumerator4
      (Default|AddtoInventory (Variables|Default|GetCharacter) "/Game/Blueprints/Interactables/1LivingRoomItems/BP_PenPencilPot.BP_PenPencilPot_C")
      (Default|CallEDItemCollected "/Game/Blueprints/Interactables/1LivingRoomItems/BP_PenPencilPot.BP_PenPencilPot_C" (Variables|Default|GetItemNameString)))
    (:NewEnumerator5
      (Default|AddtoInventory (Variables|Default|GetCharacter) "/Game/Blueprints/Interactables/1LivingRoomItems/BP_Laptop.BP_Laptop_C")
      (Default|CallEDItemCollected "/Game/Blueprints/Interactables/1LivingRoomItems/BP_Laptop.BP_Laptop_C" (Variables|Default|GetItemNameString)))
    (:NewEnumerator6
      (Default|AddtoInventory (Variables|Default|GetCharacter) "/Game/Blueprints/Interactables/2BedRoomItems/BP_Suitcase.BP_Suitcase_C")
      (Default|CallEDItemCollected "/Game/Blueprints/Interactables/2BedRoomItems/BP_Suitcase.BP_Suitcase_C" (Variables|Default|GetItemNameString)))
    (:NewEnumerator7
      (Default|AddtoInventory (Variables|Default|GetCharacter) "/Game/Blueprints/Interactables/2BedRoomItems/BP_PhoneCharger.BP_PhoneCharger_C")
      (Default|CallEDItemCollected "/Game/Blueprints/Interactables/2BedRoomItems/BP_PhoneCharger.BP_PhoneCharger_C" (Variables|Default|GetItemNameString)))
    (:NewEnumerator8
      (Default|AddtoInventory (Variables|Default|GetCharacter) "/Game/Blueprints/Interactables/2BedRoomItems/BP_Wallet.BP_Wallet_C")
      (Default|CallEDItemCollected "/Game/Blueprints/Interactables/2BedRoomItems/BP_Wallet.BP_Wallet_C" (Variables|Default|GetItemNameString)))
    (:NewEnumerator9
      (Default|AddtoInventory (Variables|Default|GetCharacter) "/Game/Blueprints/Interactables/3KitchenItems/BP_Bowl.BP_Bowl_C")
      (Default|CallEDItemCollected "/Game/Blueprints/Interactables/3KitchenItems/BP_Bowl.BP_Bowl_C" (Variables|Default|GetItemNameString)))
    (:NewEnumerator10
      (Default|AddtoInventory (Variables|Default|GetCharacter) "/Game/Blueprints/Interactables/3KitchenItems/BP_Cereal.BP_Cereal_C")
      (Default|CallEDItemCollected "/Game/Blueprints/Interactables/3KitchenItems/BP_Cereal.BP_Cereal_C" (Variables|Default|GetItemNameString)))
    (:NewEnumerator11
      (Default|AddtoInventory (Variables|Default|GetCharacter) "/Game/Blueprints/Interactables/3KitchenItems/BP_Milk.BP_Milk_C")
      (Default|CallEDItemCollected "/Game/Blueprints/Interactables/3KitchenItems/BP_Milk.BP_Milk_C" (Variables|Default|GetItemNameString)))
    (:NewEnumerator12
      (Default|AddtoInventory (Variables|Default|GetCharacter) "/Game/Blueprints/Interactables/3KitchenItems/BP_Spoon.BP_Spoon_C")
      (Default|CallEDItemCollected "/Game/Blueprints/Interactables/3KitchenItems/BP_Spoon.BP_Spoon_C" (Variables|Default|GetItemNameString)))))