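; Pickup interactable that the player collects by zooming inside its collision volume and pressing interact, earning points.
; Overlap starts a looping per-frame timer that polls zoom state, then after a delay enables interaction, lights its point light and fires dispatchers.
; Bound character dispatchers supply zoom and interact input.
; Collection adds the item to the inventory, broadcasts its name, awards points multiplied more at lower gameplay timer values, then destroys the actor.
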(event OnComponentBeginOverlap(Collision)
  (params (OverlappedComponent :type Primitive%20Component%20Object%20Reference) (OtherActor :type Actor%20Object%20Reference) (OtherComp :type Primitive%20Component%20Object%20Reference) (OtherBodyIndex :type Integer) (bFromSweep :type Boolean) (SweepResult :type Hit%20Result%20Structure%20%28by%20ref%29))
  ;[1 1 1] Begin and end overlap
  (Utilities|IsPlayerCharacter OtherActor
    (:IsPlayer
      (Variables|BaseVariables|SetInVolume true)
      (Input|EnableInput (Game|GetPlayerController 0))
      (bind _returnvalue (Utilities|Time|SetTimerbyEvent (delegate Custom|CheckZoom) (Utilities|Time|GetWorldDeltaSeconds) true))
      (Variables|BaseVariables|SetZoomTimerHandle _returnvalue))))

(event OnComponentEndOverlap(Collision)
  (params (OverlappedComponent :type Primitive%20Component%20Object%20Reference) (OtherActor :type Actor%20Object%20Reference) (OtherComp :type Primitive%20Component%20Object%20Reference) (OtherBodyIndex :type Integer))
  ;[1 1 1] Begin and end overlap
  (Utilities|IsPlayerCharacter OtherActor
    (:IsPlayer
      (Variables|BaseVariables|SetInVolume false)
      (Variables|BaseVariables|SetAbleToInteract false)
      (CallFunction|ToggleLightOff)
      (Default|CallEDCannotInteract))))

(event Custom|CanInteract
  ;[1 1 1] Interact with object if in volume and interact is pressed
  (if (Variables|BaseVariables|GetInVolume)
    (if (Variables|BaseVariables|GetAbleToInteract)
      (CallFunction|FPassItemtoCharacter)
      (Utilities|FlowControl|Delay 0.01)
      (bind _pointsincrease (CallFunction|FModifyPointsIncreaseValue))
      (Class|BPIInteractables|IPointsIncrease(Message) (Variables|Default|GetCharacter) _pointsincrease)
      (Actor|DestroyActor))))

(event Custom|ZoomDown?
  (params (IsHeld :type Boolean))
  ;[1 1 1] ZoomBindEvent
  (Variables|BaseVariables|SetCharacterZoomed IsHeld))

(event Custom|ToggleLightOn
  ;[1 1 1] Change Light Intensity
  (Rendering|Components|Light|SetIntensity (Variables|Default|GetPointLight) 5e+03))

(event Custom|ToggleLightOff
  ;[1 1 1] Change Light Intensity
  (Rendering|Components|Light|SetIntensity (Variables|Default|GetPointLight) 0.0))

(event Custom|CheckZoom
  ;[1 1 1] Begin and end overlap
  (if (Variables|BaseVariables|GetCharacterZoomed)
    (Utilities|FlowControl|Delay (Variables|Default|GetCanInteractDelay))
    (Variables|BaseVariables|SetAbleToInteract true)
    (CallFunction|ToggleLighton)
    (Default|CallEDCanInteract)
    (Default|CallEDItemType self)
    (elif (not (Variables|BaseVariables|GetInVolume))
      (Utilities|Time|ClearandInvalidateTimerbyHandle (Variables|BaseVariables|GetZoomTimerHandle))
      (CallFunction|ToggleLightOff)
      (Default|CallEDCannotInteract))))

(event EventBeginPlay
  ;[1 1 1] Begin play, get refs and bind interact
  (|CallParentFunction)
  (CallFunction|FBindings))

(fn ConstructionScript)

(fn FBindings
  (bind _character (Variables|Default|GetCharacter))
  (EventDispatchers|BindEventtoEDInteractPressed _character (EventDispatchers|CreateEvent :!event Custom|CanInteract))
  (EventDispatchers|BindEventtoEDZoomDown _character (EventDispatchers|CreateEvent :!event Custom|ZoomDown?)))

(fn FPassItemtoCharacter
  (switch Utilities|FlowControl|Switch|SwitchonE_ItemName (Variables|Default|GetItemName)
    (:NewEnumerator0
      (Default|AddtoInventory (Variables|Default|GetCharacter))
      (Default|CallEDItemCollected 0 (Variables|Default|GetItemNameString)))
    (:NewEnumerator3
      (Default|AddtoInventory (Variables|Default|GetCharacter))
      (Default|CallEDItemCollected 0 (Variables|Default|GetItemNameString)))
    (:NewEnumerator1
      (Default|AddtoInventory (Variables|Default|GetCharacter))
      (Default|CallEDItemCollected 0 (Variables|Default|GetItemNameString)))
    (:NewEnumerator4
      (Default|AddtoInventory (Variables|Default|GetCharacter))
      (Default|CallEDItemCollected 0 (Variables|Default|GetItemNameString)))
    (:NewEnumerator5
      (Default|AddtoInventory (Variables|Default|GetCharacter))
      (Default|CallEDItemCollected 0 (Variables|Default|GetItemNameString)))
    (:NewEnumerator6
      (Default|AddtoInventory (Variables|Default|GetCharacter))
      (Default|CallEDItemCollected 0 (Variables|Default|GetItemNameString)))
    (:NewEnumerator7
      (Default|AddtoInventory (Variables|Default|GetCharacter))
      (Default|CallEDItemCollected 0 (Variables|Default|GetItemNameString)))
    (:NewEnumerator8
      (Default|AddtoInventory (Variables|Default|GetCharacter))
      (Default|CallEDItemCollected 0 (Variables|Default|GetItemNameString)))
    (:NewEnumerator9
      (Default|AddtoInventory (Variables|Default|GetCharacter))
      (Default|CallEDItemCollected 0 (Variables|Default|GetItemNameString)))
    (:NewEnumerator10
      (Default|AddtoInventory (Variables|Default|GetCharacter))
      (Default|CallEDItemCollected 0 (Variables|Default|GetItemNameString)))
    (:NewEnumerator11
      (Default|AddtoInventory (Variables|Default|GetCharacter))
      (Default|CallEDItemCollected 0 (Variables|Default|GetItemNameString)))
    (:NewEnumerator12
      (Default|AddtoInventory (Variables|Default|GetCharacter))
      (Default|CallEDItemCollected 0 (Variables|Default|GetItemNameString)))))

(fn FModifyPointsIncreaseValue
  (bind _gamemoderef (Variables|Default|GetGamemodeRef))
  (bind _gameplaytimer (Variables|/Game/Blueprints/MISC/GM_SeekingComposure.GM_SeekingComposure_C|GetGameplayTimer _gamemoderef))
  (if (<= _gameplaytimer 60)
    ;[1 1 1] x4 below 1 min
    (return (* (Variables|Default|GetIncreasePoints) 4))
    (elif (<= _gameplaytimer 120)
      ;[1 1 1] x3 below 2 mins
      (return (* (Variables|Default|GetIncreasePoints) 3))
      (elif (<= _gameplaytimer 180)
        ;[1 1 1] x2 below 3 mins
        (return (* (Variables|Default|GetIncreasePoints) 2))
        (else
          ;[1 1 1] x1 above 3 mins
          (return (Variables|Default|GetIncreasePoints)))))))